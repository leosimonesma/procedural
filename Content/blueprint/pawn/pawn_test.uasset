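; Test pawn, steered by the player with Enhanced Input actions for forward motion and turning.
; On BeginPlay it adds the Mapping_base context to its player controller's input subsystem.
; Forward feeds the actor's forward vector, scaled by Vitesse, into AddMovementInput.
; Left/right and up/down apply fixed local yaw and pitch steps per input event, without delta-time scaling, so forward motion follows the pawn's orientation.
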(event Input|EnhancedActionEvents|EnhancedInputActionforward
  (params (ActionValue :type Boolean) (ElapsedSeconds :type Float%20%28double-precision%29) (TriggeredSeconds :type Float%20%28double-precision%29) (InputAction :type Input%20Action%20Object%20Reference :default "/Game/blueprint/pawn/forward.forward"))
  (Pawn|Input|AddMovementInput (* (Transformation|GetActorForwardVector) (Variables|Default|Getvitesse)) 1.0 false))

(event Input|EnhancedActionEvents|EnhancedInputActionleft
  (params (ActionValue :type Boolean) (ElapsedSeconds :type Float%20%28double-precision%29) (TriggeredSeconds :type Float%20%28double-precision%29) (InputAction :type Input%20Action%20Object%20Reference :default "/Game/blueprint/pawn/left.left"))
  (Transformation|AddActorLocalRotation "0.000000,-2.000000,0.000000" false false))

(event Input|EnhancedActionEvents|EnhancedInputActionright
  (params (ActionValue :type Boolean) (ElapsedSeconds :type Float%20%28double-precision%29) (TriggeredSeconds :type Float%20%28double-precision%29) (InputAction :type Input%20Action%20Object%20Reference :default "/Game/blueprint/pawn/right.right"))
  (Transformation|AddActorLocalRotation "0.000000,2.000000,0.000000" false false))

(event Input|EnhancedActionEvents|EnhancedInputActionup
  (params (ActionValue :type Boolean) (ElapsedSeconds :type Float%20%28double-precision%29) (TriggeredSeconds :type Float%20%28double-precision%29) (InputAction :type Input%20Action%20Object%20Reference :default "/Game/blueprint/pawn/up.up"))
  (Transformation|AddActorLocalRotation "0.500000,0.000000,0.000000" false false))

(event Input|EnhancedActionEvents|EnhancedInputActiondown
  (params (ActionValue :type Boolean) (ElapsedSeconds :type Float%20%28double-precision%29) (TriggeredSeconds :type Float%20%28double-precision%29) (InputAction :type Input%20Action%20Object%20Reference :default "/Game/blueprint/pawn/down.down"))
  (Transformation|AddActorLocalRotation "-0.500000,0.000000,0.000000" false false))

(event EventBeginPlay
  (bind _asplayer_controller (Utilities|Casting|CastToPlayerController (Pawn|GetController)))
  (Utilities|IsValid (PlayerController|LocalPlayerSubsystems|GetEnhancedInputLocalPlayerSubsystem _asplayer_controller)
    (:Is%20Valid
      (Input|AddMappingContext (PlayerController|LocalPlayerSubsystems|GetEnhancedInputLocalPlayerSubsystem _asplayer_controller) "/Game/blueprint/pawn/mapping_base.mapping_base" 0 "(bIgnoreAllPressedKeysUntilRelease=True,bForceImmediately=False,bNotifyUserSettings=False)"))))

(event Collision|EventActorBeginOverlap
  (params (OtherActor :type Actor%20Object%20Reference)))

(event EventTick
  (params (DeltaSeconds :type Float%20%28single-precision%29)))

(fn ConstructionScript)