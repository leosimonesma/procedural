(event Custom|Generation
  (params (STR_Ref :type Array%20of%20STR%20Correspondance%20Structures) (Nb_Rota :type Integer))
  (bind _tuiles_generated (Variables|Default|GetTuiles_Generated))
  (bind _tuiles_generated_2 (Variables|Default|GetTuiles_Generated))
  (bind _returnvalue (Utilities|Array|LastIndex _tuiles_generated))
  (bind _output (Utilities|Array|Get(acopy) _tuiles_generated _returnvalue))
  (bind _returnvalue_2 (Transformation|GetActorLocation _output))
  (for _index (range 1 Nb_Rota)
    (bind _returnvalue_3 (Game|SpawnActorfromClass (Utilities|Array|Get(acopy) (Variables|Default|GetRef_Tuiles) (.OutItem (Utilities|Array|Random (.correspondance (Utilities|Array|Get(acopy) STR_Ref (Variables|/Game/Methode_01/BP_TUILE_PARENT.BP_TUILE_PARENT_C|GetID (Utilities|Array|Get(acopy) _tuiles_generated_2 (Utilities|Array|LastIndex _tuiles_generated_2)))))))) (Math|Transform|MakeTransform (Math|Vector|MakeVector (+ 1e+04 (.x _returnvalue_2)) (.y _returnvalue_2) (.z _returnvalue_2)) "0, 0, 0" "1.000000,1.000000,1.000000") "Undefined" "MultiplyWithRoot" 0 0))
    (Utilities|Array|Add (Variables|Default|GetTuiles_Generated) _returnvalue_3)))

(event Custom|Create
  (bind _ref_tuiles (Variables|Default|GetRef_Tuiles))
  (bind _returnvalue (Game|SpawnActorfromClass (Utilities|Array|Get(acopy) _ref_tuiles (.OutIndex (Utilities|Array|Random _ref_tuiles))) (Math|Transform|MakeTransform "0.0,0.0,0.0" "0, 0, 0" "1.000000,1.000000,1.000000") "Undefined" "MultiplyWithRoot" 0 0))
  (Utilities|Array|Add (Variables|Default|GetTuiles_Generated) _returnvalue))

(event EventBeginPlay)

(event Collision|EventActorBeginOverlap
  (params (OtherActor :type Actor%20Object%20Reference)))

(event EventTick
  (params (DeltaSeconds :type Float%20%28single-precision%29)))

(fn ConstructionScript)

(fn FillDataTable
  (for _array_element (Variables|Default|GetTuiles_Generated)
    (if (Variables|Default|GetFirst)
      (Variables|Default|SetDebut_nom (Utilities|String|Append (Variables|Default|GetFirst_line) " 
" (Utilities|GetClassDisplayName (Utilities|GetClass _array_element)) ",\"" (Utilities|String|ToString(Integer) (Variables|/Game/Methode_01/BP_TUILE_PARENT.BP_TUILE_PARENT_C|GetID _array_element)) "\",\"(x=" (Utilities|String|ToString(Float) (.x (Transformation|GetActorLocation _array_element))) ",y=" (Utilities|String|ToString(Float) (.y (Transformation|GetActorLocation _array_element))) ",z=" (Utilities|String|ToString(Float) (.z (Transformation|GetActorLocation _array_element))) ")\"" " 
"))
      (Variables|Default|SetFirst false)
      (else
        (Variables|Default|SetDebut_nom (Utilities|String|Append (Variables|Default|GetDebut_nom) (Utilities|GetClassDisplayName (Utilities|GetClass _array_element)) ",\"" (Utilities|String|ToString(Integer) (Variables|/Game/Methode_01/BP_TUILE_PARENT.BP_TUILE_PARENT_C|GetID _array_element)) "\",\"(x=" (Utilities|String|ToString(Float) (.x (Transformation|GetActorLocation _array_element))) ",y=" (Utilities|String|ToString(Float) (.y (Transformation|GetActorLocation _array_element))) ",z=" (Utilities|String|ToString(Float) (.z (Transformation|GetActorLocation _array_element))) ")\"" " 
")))))
  (return (Variables|Default|GetDebut_nom)))