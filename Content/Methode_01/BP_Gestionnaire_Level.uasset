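; Level manager that spawns track tiles on request and caps how many stay in the world.
; Appel_construction_Tuiles looks up the requested TypeTile in the StrucRef array and spawns each matching class at a fixed forward X offset from Pos.
; Spawned tiles queue in TuilesGenerated, which destroys its oldest entry beyond ten, forming a rolling window of level pieces.
; Spawn_tile and the construction script are empty.
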(event Custom|Appel_construction_Tuiles
  (params (Pos :type Vector) (Type_Tile :type Integer))
  (Variables|Default|SetType%20Tile Type_Tile)
  (for _array_element (Variables|Default|GetStruc_Ref)
    (if (== (.membervar_0 _array_element) (Variables|Default|GetType%20Tile))
      (bind _returnvalue (Game|SpawnActorfromClass (.membervar_1 _array_element) (Math|Transform|MakeTransform (Math|Vector|MakeVector (+ 1e+04 (.x Pos)) (.y Pos) (.z Pos)) "0, 0, 0" "1.000000,1.000000,1.000000") "Undefined" "MultiplyWithRoot" 0 0))
      (Utilities|Array|Add (Variables|Default|GetTuiles_Generated) _returnvalue)
      (if (> (Utilities|Array|Length (Variables|Default|GetTuiles_Generated)) 10)
        (Actor|DestroyActor (Utilities|Array|Get(acopy) (Variables|Default|GetTuiles_Generated)))
        (Utilities|Array|RemoveIndex (Variables|Default|GetTuiles_Generated))))))

(event Custom|Spawn_tile
  ;[0.15 0.15 0.15 0.5] BP_tile_1
)

(fn ConstructionScript)