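; BP_TUILE_PARENT is a parent tile Blueprint that requests construction of a compatible tile when its Box is overlapped.
; On BeginPlay it retrieves the level manager reference from my_game_mode, retrying after a short delay until it is valid.
; The first overlap, gated by DoOnce, shuffles ListTuilesCompatibles and passes its first entry and the tile's location to the manager's AppelConstructionTuiles.
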(event OnComponentBeginOverlap(Box)
  (params (OverlappedComponent :type Primitive%20Component%20Object%20Reference) (OtherActor :type Actor%20Object%20Reference) (OtherComp :type Primitive%20Component%20Object%20Reference) (OtherBodyIndex :type Integer) (bFromSweep :type Boolean) (SweepResult :type Hit%20Result%20Structure%20%28by%20ref%29))
  (Development|PrintString "Hello")
  (Utilities|FlowControl|DoOnce false
    (:Completed
      (Utilities|Array|Shuffle (Variables|Default|GetList_Tuiles_Compatibles))
      (Default|AppelConstructionTuiles (Variables|Default|GetRef%20Gestionnaire%20Lvl) (Transformation|GetActorLocation) (Utilities|Array|Get(acopy) (Variables|Default|GetList_Tuiles_Compatibles)))
      (Variables|Default|SetSpawned false))))

(event EventBeginPlay
  (bind _asmy_game_mode (Utilities|Casting|CastTomy_game_mode (Game|GetGameMode)))
  (bind _output_get (Variables|Default|SetRef%20Gestionnaire%20Lvl (Variables|/Game/blueprint/management/my_game_mode.my_game_mode_C|GetRef_Gestionnaire_Lvl _asmy_game_mode) :!label _label))
  (Utilities|IsValid _output_get
    (:Is%20Not%20Valid
      (Utilities|FlowControl|Delay 0.01)
      (goto _label))))

(fn ConstructionScript)